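; Enemy laser turret that turns toward a seen first-person player, charges for three seconds, then fires a beam for five seconds.
; PawnSensing drives the aim, charge and end sounds, and state flags, with aim locked while firing.
; A per-tick line trace measures wall distance to stretch the laser mesh's X scale.
; Tick also runs a timeline tinting the Sphere's dynamic material while ChangeColor is set, otherwise resetting it to white.
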(event `self.ReceiveBeginPlay`
  ;[1 0 0.8672] Change Color Material
  (bind _returnvalue (`PrimitiveComponent.CreateDynamicMaterialInstance` (`self.Sphere`) 0 "/Game/AlexScenes/Matterials/GlowEnemyShoot_Mat.GlowEnemyShoot_Mat" "None"))
  (set `self.MaterialLaser` _returnvalue)
  (if (`self.PlayerAdquired`)
    (`/Engine/EditorBlueprintResources/StandardMacros.DoOnce` false :!label _label
      (:`Completed`
        (bind (_direction _newtrack_0) (`Timeline|Timeline_0` :!via `PlayFromStart`)
          (:`Update`
            (bind _output_get (set `self.Value` (make `LinearColor` 1.0 _newtrack_0 _newtrack_0 1.0)))
            (`MaterialInstanceDynamic.SetVectorParameterValue` _returnvalue "None" _output_get)))))
    (else
      (`|ExecutionSequence`
        (:`then_0`
          (goto _label :!via `Reset`))
        (:`then_1`
          (`MaterialInstanceDynamic.SetVectorParameterValue` _returnvalue "None" (struct :`R` 1.0 :`G` 1.0 :`B` 1.0 :`A` 1.0)))))))

(event `self.PawnSensing.OnSeePawn`
  (params (Pawn :type "Pawn Object Reference"))
  (bind _laserbeam_sound (`self.LaserBeam_Sound`))
  (bind _laserbeam_sound_2 (`self.LaserBeam_Sound`))
  ;[1 0.7266 0] Shooting Laser Beam
  (bind _asfirst_person_character (cast `/Game/FirstPersonBP/Blueprints/FirstPersonCharacter` Pawn))
  (`|ExecutionSequence`
    (:`then_0`
      (if (not (`self.PlayerAdquired`))
        (`self.K2_SetActorRotation` (`KismetMathLibrary.FindLookAtRotation` (`self.K2_GetActorLocation`) (`self.K2_GetActorLocation` _asfirst_person_character)))
        (if (not (`self.ChangeColor`))
          (`KismetSystemLibrary.Delay` 0.1)
          (set `self.ChangeColor` true)
          (`AudioComponent.Stop` _laserbeam_sound)
          (`AudioComponent.SetSound` _laserbeam_sound "/Game/AlexScenes/Sounds/LaserBeam_Start.LaserBeam_Start")
          (`AudioComponent.Play` _laserbeam_sound 0.0)
          (`KismetSystemLibrary.Delay` 3.0)
          (set `self.PlayerAdquired` true))))
    (:`then_1`
      (if (`self.PlayerAdquired`)
        (`|ExecutionSequence`
          (:`then_0`
            (`/Engine/EditorBlueprintResources/StandardMacros.DoOnce` false :!label _label_2
              (:`Completed`
                (`AudioComponent.SetSound` _laserbeam_sound_2 "/Game/AlexScenes/Sounds/LaserBeam_End.LaserBeam_End")
                (`AudioComponent.Play` _laserbeam_sound_2 0.0))))
          (:`then_1`
            (`SceneComponent.SetRelativeScale3D` (`self.Laser`) (`KismetMathLibrary.MakeVector` (/ (`self.DistanceToWall`) 50.0) 0.13 0.13))
            (`KismetSystemLibrary.Delay` 5.0)
            (`SceneComponent.SetRelativeScale3D` (`self.Laser`) (0.13 0.13 0.13))
            (set `self.PlayerAdquired` false)
            (goto _label_2 :!via `Reset`)))))))

(event `self.ReceiveTick`
  (params (DeltaSeconds :type "Float (single-precision)"))
  (bind _materiallaser (`self.MaterialLaser`))
  (bind _laser (`self.Laser`))
  (bind _returnvalue (`SceneComponent.K2_GetComponentLocation` _laser))
  ;[0 1 0.8359] Laser Lenght
  (bind _outhit (`KismetSystemLibrary.LineTraceSingle` _returnvalue (+ _returnvalue (* (`SceneComponent.GetForwardVector` _laser) 10000.0)) "TraceTypeQuery1"))
  (set `self.DistanceToWall` (`.Distance` (`GameplayStatics.BreakHitResult` _outhit)))
  ;[0 0.01562 1] Laser Change Material Colo in Run Time
  (if (`self.ChangeColor`)
    (`/Engine/EditorBlueprintResources/StandardMacros.DoOnce` false :!label _label_3
      (:`Completed`
        (bind (_direction _newtrack_0) (`Timeline|Timeline_1` :!via `PlayFromStart`)
          (:`Update`
            (bind _output_get (set `self.Value` (make `LinearColor` 1.0 _newtrack_0 _newtrack_0 1.0)))
            (`MaterialInstanceDynamic.SetVectorParameterValue` _materiallaser "Color" _output_get)
            (`KismetSystemLibrary.Delay` 8.0)
            (set `self.ChangeColor` false)))))
    (else
      (`|ExecutionSequence`
        (:`then_0`
          (goto _label_3 :!via `Reset`))
        (:`then_1`
          (`MaterialInstanceDynamic.SetVectorParameterValue` _materiallaser "Color" (struct :`R` 1.0 :`G` 1.0 :`B` 1.0 :`A` 1.0)))))))

(fn `UserConstructionScript`)