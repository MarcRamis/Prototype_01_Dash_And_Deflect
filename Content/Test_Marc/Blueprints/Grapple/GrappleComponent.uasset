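; Grappling hook component for the first-person character that pulls the player toward grapple target actors.
; A Tick-driven state machine, while retracted, highlights the visible in-range target closest in angle to the camera's forward vector.
; AttemptGrapple spawns a hook and a cable line attached to the left hand.
; As the hook nears, the character hops, flies toward the target from the apex, then gets a final launch before cleanup.
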(event `self.ReceiveBeginPlay`
  (bind _asfirst_person_character (cast `/Game/FirstPersonBP/Blueprints/FirstPersonCharacter` (`self.GetOwner`)))
  (set `self.OurCharacter` _asfirst_person_character))

(event `self.ReceiveTick`
  (params (DeltaSeconds :type "Float (single-precision)"))
  (switch `/Game/Test_Marc/Blueprints/Grapple/EGrappleState` (`self.GrappleState`)
    (:`NewEnumerator0`
      (`self.TickRetracted`))
    (:`NewEnumerator1`
      (`self.TickFiring`))
    (:`NewEnumerator2`
      (`self.TickNearingTarget`))
    (:`NewEnumerator3`
      (`self.TickOnTarget`))))

(fn `AttemptGrapple`
  (switch `/Game/Test_Marc/Blueprints/Grapple/EGrappleState` (`self.GrappleState`)
    (:`NewEnumerator0`
      (bind _currenttarget (`self.CurrentTarget`)
        (:`then`
          (bind _returnvalue (`|SpawnActorFromClass` "/Game/Test_Marc/Blueprints/Grapple/BP_GrappleHook.BP_GrappleHook_C" (`KismetMathLibrary.MakeTransform` (`self.OwnerLocation`)) "AlwaysSpawn" "OverrideRootScale" null _currenttarget 5000.0 null))
          (set `self.GrappleHook` _returnvalue)
          (bind _returnvalue_2 (`|SpawnActorFromClass` "/Game/Test_Marc/Blueprints/Grapple/BP_GrappleLine.BP_GrappleLine_C" (`KismetMathLibrary.MakeTransform` (`self.OwnerLocation`)) "AlwaysSpawn" "OverrideRootScale" null null))
          (bind _output_get (set `self.GrappleLine` _returnvalue_2))
          (`Actor.K2_AttachToComponent` _output_get (`/Game/FirstPersonBP/Blueprints/FirstPersonCharacter.Mesh2P` (`self.OurCharacter`)) "hand_l" "SnapToTarget" "SnapToTarget" "SnapToTarget" true)
          (`CableComponent.SetAttachEndTo` (`CableActor.CableComponent` (`self.GrappleLine`)) (`self.GrappleHook`) "DefaultSceneRoot" "None")
          (set `self.GrappleState` "NewEnumerator1"))
        (:`else`)))))

(fn `DestroyGrappleComponents`
  (`Actor.K2_DestroyActor` (`self.GrappleLine`))
  (set `self.GrappleLine` null)
  (`Actor.K2_DestroyActor` (`self.GrappleHook`))
  (set `self.GrappleHook` null)
  (set `self.GrappleState` "NewEnumerator0"))

(fn `FindBestTarget`
  (params (Targets :type "Array of Actor Object Reference"))
  (returns (Target :type "Actor Object Reference"))
  (locals (`CurrentTarget (local)` :type "Actor Object Reference") (`CurrentAngle (local)` :type "Float (double-precision)" :default 0.0) (`BestAngle (local)` :type "Float (double-precision)") (`BestTarget (local)` :type "Actor Object Reference"))
  (bind _ourcharacter (`self.OurCharacter`))
  (for _array_element Targets
    (set `local.CurrentTarget (local)` _array_element)
    (bind (_outhit _returnvalue) (`KismetSystemLibrary.LineTraceSingle` (`Actor.K2_GetActorLocation` (`self.OurCharacter`)) (`Actor.K2_GetActorLocation` (`local.CurrentTarget (local)`)) "TraceTypeQuery1" false (`|MakeArray` (`self.OurCharacter`) :!type "Actor Object Reference") "None" true (struct :`R` 1.0 :`A` 1.0) (struct :`G` 1.0 :`A` 1.0) 0.2))
    (if _returnvalue
      (if (== (`.HitActor` (`GameplayStatics.BreakHitResult` _outhit)) (`local.CurrentTarget (local)`))
        (`|ExecutionSequence`
          (:`then_0`
            ;[0 0.6719 1] Calculate the angle to the target
            (set `local.CurrentAngle (local)` (`KismetMathLibrary.DegAcos` (`KismetMathLibrary.Dot_VectorVector` (`KismetMathLibrary.Normal` (- (`Actor.K2_GetActorLocation` (`local.CurrentTarget (local)`)) (`Actor.K2_GetActorLocation` _ourcharacter))) (`SceneComponent.GetForwardVector` (`/Game/FirstPersonBP/Blueprints/FirstPersonCharacter.FirstPersonCamera` _ourcharacter))))))
          (:`then_1`
            ;[0 1 0.3438] If the angle is less than our current angle make this our new target
            (if (or (< (`local.CurrentAngle (local)`) (`local.BestAngle (local)`)) (not (`KismetSystemLibrary.IsValid` (`local.BestTarget (local)`))))
              (set `local.BestTarget (local)` (`local.CurrentTarget (local)`))
              (set `local.BestAngle (local)` (`local.CurrentAngle (local)`))))))))
  (return (`local.BestTarget (local)`)))

(fn `SetCurrentTarget`
  (params (`\`NewTarget` :type "/Game/Test_Marc/Blueprints/Grapple/BP_GrappleTarget Object Reference"))
  (if (!= `\`NewTarget` (`self.CurrentTarget`))
    (`|ExecutionSequence`
      (:`then_0`
        (bind _currenttarget (`self.CurrentTarget`)
          (:`then`
            (`/Game/Test_Marc/Blueprints/Grapple/BP_GrappleTarget.SetActive` _currenttarget false))
          (:`else`)))
      (:`then_1`
        (set `self.CurrentTarget` (`local.\`NewTarget`)))
      (:`then_2`
        (bind _currenttarget_2 (`self.CurrentTarget`)
          (:`then`
            (`/Game/Test_Marc/Blueprints/Grapple/BP_GrappleTarget.SetActive` _currenttarget_2 true))
          (:`else`))))))

(fn `TickFiring`
  (if (< (`/Game/Test_Marc/Blueprints/Grapple/BP_GrappleHook.DistanceToTarget` (`self.GrappleHook`)) (`self.StartJumpDistance`))
    (`Character.LaunchCharacter` (`self.OurCharacter`) (0.0 0.0 500.0) true true)
    (set `self.GrappleState` "NewEnumerator2")))

(fn `TickNearingTarget`
  (bind (_returnvalue_x _returnvalue_y _returnvalue_z) (`KismetMathLibrary.BreakVector` (`Actor.GetVelocity` (`self.OurCharacter`))))
  (if (<= _returnvalue_z 0.0)
    (set `self.InitialDirection` (`self.OwnerToTarget`))
    (`self.Activate` (`/Game/FirstPersonBP/Blueprints/FirstPersonCharacter.GrappleLines` (`self.OurCharacter`)) false)
    (`GameplayStatics.PlaySoundAtLocation` "/Game/Test_Marc/Audios/S_Grappling.S_Grappling" (`Actor.K2_GetActorLocation` (`self.OurCharacter`)) (struct) 1.0 1.0 0.0 null null null)
    (set `self.GrappleState` "NewEnumerator3")))

(fn `TickOnTarget`
  (bind (_returnvalue_x _returnvalue_y _returnvalue_z) (`KismetMathLibrary.BreakVector` (* (`self.InitialDirection`) 100.0)))
  (if (< (`Actor.GetDistanceTo` (`self.OurCharacter`) (`self.CurrentTarget`)) (`self.EndJumpDistance`))
    (set `self.IsGrappeling` true)
    (`Character.LaunchCharacter` (`self.OurCharacter`) (`KismetMathLibrary.MakeVector` _returnvalue_x _returnvalue_y (`KismetMathLibrary.FMax` _returnvalue_z 500.0)) true true)
    (`self.SetCurrentTarget` null)
    (set `self.IsGrappeling` false)
    (`self.DestroyGrappleComponents`)
    (else
      (set `MovementComponent.Velocity` (* (`self.OwnerToTarget`) (`self.CharacterGrappleSpeed`)) (`Pawn.GetMovementComponent` (`self.OurCharacter`))))))

(fn `TickRetracted`
  (bind _outactors (`KismetSystemLibrary.SphereOverlapActors` (`Actor.K2_GetActorLocation` (`self.OurCharacter`)) (`self.MaxGrappleDistance`) (`|MakeArray` "ObjectTypeQuery1" :!type "EObjectTypeQuery Enum") "/Game/Test_Marc/Blueprints/Grapple/BP_GrappleTarget.BP_GrappleTarget_C"))
  (bind _target (`self.FindBestTarget` _outactors))
  (`self.SetCurrentTarget` (cast `/Game/Test_Marc/Blueprints/Grapple/BP_GrappleTarget` _target :!pure true)))